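; BP_Checkpoint is a checkpoint actor that saves the chicken player's progress when it overlaps the hit box.
; Each such overlap calls SaveCheckpoint on BP_ChickenPlayer and plays a bell-spoon sound at the actor, with a delayed stop.
; The glow ring starts hidden; the first activation reveals it and a timeline grows its Z scale, with GlowVis guarding against replays.
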(event OnComponentBeginOverlap(checkPointHitBox)
  (params (OverlappedComponent :type Primitive%20Component%20Object%20Reference) (OtherActor :type Actor%20Object%20Reference) (OtherComp :type Primitive%20Component%20Object%20Reference) (OtherBodyIndex :type Integer) (bFromSweep :type Boolean) (SweepResult :type Hit%20Result%20Structure%20%28by%20ref%29))
  (bind _sm_fx_glow_ring_01 (Variables|Default|GetSM_FX_Glow_Ring_01))
  (bind _relativescale3d (Variables|/Script/Engine.SceneComponent|GetRelativeScale3D _sm_fx_glow_ring_01))
  (bind _asbp_chicken_player (Utilities|Casting|CastToBP_ChickenPlayer OtherActor))
  (Default|SaveCheckpoint _asbp_chicken_player)
  (bind _returnvalue (Audio|SpawnSoundatLocation "/Game/Audio/FX/Toys/BellSpoon.BellSpoon" (Transformation|GetWorldLocation (Variables|Default|GetDefaultSceneRoot)) "0, 0, 0" 4.0 1.0 0.0 0 0))
  (Audio|Components|Audio|Play _returnvalue 0.0)
  (Audio|Components|Audio|StopDelayed _returnvalue 5.0)
  (if (not (Variables|Default|GetglowVis))
    (Rendering|SetVisibility (Variables|Default|GetSM_FX_Glow_Ring_01) true false)
    (bind _newtrack_0 (Timeline|Timeline_0 PlayFromStart)
      (:Update
        (Transformation|SetRelativeScale3D _sm_fx_glow_ring_01 (Math|Vector|MakeVector (.x _relativescale3d) (.y _relativescale3d) (Math|Float|Lerp 0.0 1.5 _newtrack_0)))
        (Variables|Default|SetglowVis true)))))

(event EventBeginPlay
  (Rendering|SetVisibility (Variables|Default|GetSM_FX_Glow_Ring_01) false false))

(event Collision|EventActorBeginOverlap
  (params (OtherActor :type Actor%20Object%20Reference)))

(event EventTick
  (params (DeltaSeconds :type Float%20%28single-precision%29)))

(fn ConstructionScript)