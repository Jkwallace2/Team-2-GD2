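; BP_Collectable is a floating pickup that can act as a coin, an egg or a generic item.
; A timeline with a randomized start time bobs and spins it, with an optional looping-style ambient sound.
; Collect, an externally triggered event, increments the matching BP_ChickenPlayer counter, disables collision and plays a pickup sound.
; A second timeline pulls it toward the player while shrinking, fading and pitch-shifting the sound, then destroys it.
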(event Custom|Collect
  (bind _returnvalue (Game|Player|GetPlayerPawn 0))
  (bind _ambientsound (Variables|Default|GetAmbientSound))
  (bind _returnvalue_2 (Transformation|GetActorLocation _returnvalue))
  (if (Variables|Default|GetisCoin)
    (Utilities|FlowControl|DoOnce false
      (:Completed
        (bind _asbp_chicken_player (Utilities|Casting|CastToBP_ChickenPlayer (Game|Player|GetPlayerPawn 0)))
        (bind _output_get (Variables|/Game/ChickenGame/BluePrints/BP_ChickenPlayer.BP_ChickenPlayer_C|SetCoinValue _asbp_chicken_player (+ (Variables|/Game/ChickenGame/BluePrints/BP_ChickenPlayer.BP_ChickenPlayer_C|GetCoinValue _asbp_chicken_player) 1.0)))
        (Development|PrintString (Utilities|String|Append "New coin value: " (Utilities|String|ToString(Float) _output_get)))))
    (elif (Variables|Default|GetisEgg)
      (Utilities|FlowControl|DoOnce false
        (:Completed
          (bind _asbp_chicken_player_2 (Utilities|Casting|CastToBP_ChickenPlayer (Game|Player|GetPlayerPawn 0)))
          (bind _output_get_2 (Variables|/Game/ChickenGame/BluePrints/BP_ChickenPlayer.BP_ChickenPlayer_C|SetEggValue _asbp_chicken_player_2 (+ (Variables|/Game/ChickenGame/BluePrints/BP_ChickenPlayer.BP_ChickenPlayer_C|GetEggValue _asbp_chicken_player_2) 1.0)))
          (Development|PrintString (Utilities|String|Append "New egg value: " (Utilities|String|ToString(Float) _output_get_2)))))
      (else
        (Utilities|FlowControl|DoOnce false
          (:Completed
            _)))))
  (Utilities|FlowControl|Sequence
    (:then_1
      (Collision|SetCollisionEnabled (Variables|Default|GetCapsule) "NoCollision")
      (Audio|PlaySoundatLocation (Variables|Sound|GetPickupSound) _returnvalue_2 "0, 0, 0" 1.0 1.0 0.0 0 0 0 0)
      (bind _newtrack_1 (Timeline|Timeline_0 PlayFromStart)
        (:Update
          (Transformation|SetWorldLocation (Variables|Default|GetDefaultSceneRoot) (Math|Vector|Lerp(Vector) (Transformation|GetWorldLocation (Variables|Default|GetDefaultSceneRoot)) _returnvalue_2 _newtrack_1) false false)
          (Transformation|SetRelativeScale3D (Variables|Default|GetDefaultSceneRoot) (Math|Conversions|ToVector(Float) (- 1.0 _newtrack_1)))
          (Audio|Components|Audio|SetVolumeMultiplier _ambientsound (* (- 1.0 _newtrack_1) (Variables|Sound|GetFloat%20Volume)) :!class /Script/Engine.AudioComponent)
          (Audio|Components|Audio|SetPitchMultiplier _ambientsound (+ (Variables|Sound|GetFloat%20pitch) (* _newtrack_1 0.5)))
          (Variables|Default|SetisEgg false)
          (Variables|Default|SetisCoin false))
        (:Finished
          (Audio|Components|Audio|Stop (Variables|Default|GetAmbientSound))
          (Actor|DestroyActor))))))

(event Custom|settime
  (bind (_direction _newtrack_1 _newtrack_2) (Timeline|Timeline SetNewTime)
    (:Update
      (Transformation|SetRelativeLocation (Variables|Default|Getoffset) (Math|Vector|MakeVector 0.0 0.0 (+ (* _newtrack_1 (Variables|Default|GetSinePower)) (Variables|Default|GetZoffset))) false false)
      (Transformation|SetRelativeRotation (Variables|Default|Getoffset) (Math|Rotator|MakeRotator 0.0 0.0 (* _newtrack_2 3.6e+02)) false false))))

(event EventBeginPlay
  (bind _ambientsound (Variables|Default|GetAmbientSound))
  (if (Variables|Sound|GetHasFloatingSound)
    (Audio|Components|Audio|Play _ambientsound 0.0)
    (Audio|Components|Audio|SetVolumeMultiplier _ambientsound (Variables|Sound|GetFloat%20Volume) :!class /Script/Engine.AudioComponent))
  (Variables|Default|SetZoffset (.z (Variables|/Script/Engine.SceneComponent|GetRelativeLocation (Variables|Default|Getoffset))))
  (CallFunction|Settime)
  (bind (_direction _newtrack_1 _newtrack_2) (Timeline|Timeline Play)
    (:Update
      (Transformation|SetRelativeLocation (Variables|Default|Getoffset) (Math|Vector|MakeVector 0.0 0.0 (+ (* _newtrack_1 (Variables|Default|GetSinePower)) (Variables|Default|GetZoffset))) false false)
      (Transformation|SetRelativeRotation (Variables|Default|Getoffset) (Math|Rotator|MakeRotator 0.0 0.0 (* _newtrack_2 3.6e+02)) false false))))

(event Collision|EventActorBeginOverlap
  (params (OtherActor :type Actor%20Object%20Reference)))

(fn ConstructionScript
  (bind _ambientsound (Variables|Default|GetAmbientSound))
  (Audio|Components|Audio|SetSound _ambientsound (Variables|Sound|GetFloating%20Sound))
  (Audio|Components|Audio|SetPitchMultiplier _ambientsound (Variables|Sound|GetFloat%20pitch)))