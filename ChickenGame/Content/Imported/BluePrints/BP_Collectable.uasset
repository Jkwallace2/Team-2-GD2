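; Collectable pickup that bobs and spins until the first-person character touches it, then flies into the player and vanishes.
; A timeline drives the idle height and yaw of the Offset component, with a random value apparently intended to stagger its phase.
; Capsule overlap, behind a DoOnce, calls the character's TakeDamage with a negative amount, disables collision and plays a coin sound.
; A second timeline lerps the root toward the player's current location while shrinking it, then destroys the actor.
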(event OnComponentBeginOverlap(Capsule)
  (params (OverlappedComponent :type Primitive%20Component%20Object%20Reference) (OtherActor :type Actor%20Object%20Reference) (OtherComp :type Primitive%20Component%20Object%20Reference) (OtherBodyIndex :type Integer) (bFromSweep :type Boolean) (SweepResult :type Hit%20Result%20Structure%20%28by%20ref%29))
  (Utilities|FlowControl|DoOnce false
    (:Completed
      (bind _asbp_first_person_character (Utilities|Casting|CastToBP_FirstPersonCharacter OtherActor))
      (Default|TakeDamage _asbp_first_person_character -1)
      (Collision|SetCollisionEnabled (Variables|Default|GetCapsule) "NoCollision")
      (Audio|PlaySoundatLocation "/Game/Imported/Audio/FX/Toys/coin.coin" (Transformation|GetActorLocation _asbp_first_person_character) "0, 0, 0" 3.0 1.0 0.0 0 0 0 0)
      (bind _newtrack_1 (Timeline|Timeline_0 PlayFromStart)
        (:Update
          (Transformation|SetWorldLocation (Variables|Default|GetDefaultSceneRoot) (Math|Vector|Lerp(Vector) (Transformation|GetWorldLocation (Variables|Default|GetDefaultSceneRoot)) (Transformation|GetActorLocation _asbp_first_person_character) _newtrack_1) false false)
          (Transformation|SetRelativeScale3D (Variables|Default|GetDefaultSceneRoot) (Math|Conversions|ToVector(Float) (- 1.0 _newtrack_1))))
        (:Finished
          (Actor|DestroyActor))))))

(event Custom|settime
  (bind (_direction _newtrack_1 _newtrack_2) (Timeline|Timeline SetNewTime)
    (:Update
      (Transformation|SetRelativeLocation (Variables|Default|Getoffset) (Math|Vector|MakeVector 0.0 0.0 (+ (* _newtrack_1 2e+01) (Variables|Default|GetZoffset))) false false)
      (Transformation|SetRelativeRotation (Variables|Default|Getoffset) (Math|Rotator|MakeRotator 0.0 0.0 (* _newtrack_2 3.6e+02)) false false))))

(event EventBeginPlay
  (Variables|Default|SetZoffset (.z (Variables|/Script/Engine.SceneComponent|GetRelativeLocation (Variables|Default|Getoffset))))
  (CallFunction|Settime)
  (bind (_direction _newtrack_1 _newtrack_2) (Timeline|Timeline Play)
    (:Update
      (Transformation|SetRelativeLocation (Variables|Default|Getoffset) (Math|Vector|MakeVector 0.0 0.0 (+ (* _newtrack_1 2e+01) (Variables|Default|GetZoffset))) false false)
      (Transformation|SetRelativeRotation (Variables|Default|Getoffset) (Math|Rotator|MakeRotator 0.0 0.0 (* _newtrack_2 3.6e+02)) false false))))

(event Collision|EventActorBeginOverlap
  (params (OtherActor :type Actor%20Object%20Reference)))

(fn ConstructionScript)