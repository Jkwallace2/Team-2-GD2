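; Enemy character that chases the player, makes a squash-and-stretch hop attack and shrinks as it loses health.
; A looping AIMoveTo triggers Attack on success or teleports a small random offset on failure, then retries.
; Attack uses timelines to hop and deform the mesh, damaging the player if within melee range afterwards.
; TakeDamage spawns mud effects and gore sounds, rescales the mesh by remaining health, and destroys the actor at zero.
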(event Custom|TakeDamage
  (params (DamageColor :type Enum_Colors%20Enum :default "NewEnumerator0") (DamageAmount :type Integer) (Location :type Vector))
  ;[0.15 0.15 0.15 0.5] Health and damage
  (Variables|Default|SetDamage%20Amount DamageAmount)
  (Variables|Default|SetLocation Location)
  (Niagara|SpawnSystematLocation "/Game/SEPP/NS_MudSquirt.NS_MudSquirt" (Variables|Default|GetLocation))
  (Audio|PlaySoundatLocation "/Game/Imported/Audio/FX/Cantaloupe/Cantaloupe_Gore2.Cantaloupe_Gore2" (Variables|Default|GetLocation) "0, 0, 0" 0.4 1.0 0.0 0 0 0 0)
  (Variables|Default|SetLocalhealth (- (Variables|Default|GetLocalhealth) (Variables|Default|GetDamage%20Amount)))
  (CallFunction|UpdateHealth))

(event Custom|UpdateHealth
  ;[0.15 0.15 0.15 0.5] Health and damage
  (Transformation|SetRelativeScale3D (Variables|Default|GetStaticMesh) (Math|Vector|Lerp(Vector) (Variables|Default|GetMin%20Scale) (Variables|Default|GetMaxScale) (Math|Float|MapRangeClamped (Math|Conversions|ToFloat(Integer) (Variables|Default|GetLocalhealth)) 0.0 (Math|Conversions|ToFloat(Integer) (Variables|Default|GetHealth)) 0.0 1.0)))
  (if (<= (Variables|Default|GetLocalhealth) 0)
    (CallFunction|Predie)))

(event Custom|Die
  (Variables|Default|SetCan%20Attack false)
  (Niagara|SpawnSystematLocation "/Game/SEPP/NS_MudSlpat.NS_MudSlpat" (Variables|Default|GetLocation))
  (Audio|PlaySoundatLocation "/Game/Imported/Audio/FX/Cantaloupe/Cantaloupe_Gore1.Cantaloupe_Gore1" (Variables|Default|GetLocation) "0, 0, 0" 1.0 1.0 0.0 0 0 0 0)
  (Utilities|FlowControl|Delay 0.01)
  (Development|PrintString (Utilities|GetDisplayName (Variables|Default|GetManager)))
  (Actor|DestroyActor))

(event Custom|Dumb%20player%20follow
  (bind _returnvalue (Math|Random|RandomIntegerinRange 20 50))
  (bind _self self)
  (bind _mesh (Variables|Character|GetMesh _self))
  (AI|AIMoveTo self "0, 0, 0" (Game|GetPlayerCharacter 0) 5.0 false
    (:OnSuccess
      (CallFunction|Attack)
      (Utilities|FlowControl|Delay 2.0))
    (:OnFail
      (Transformation|Teleport (+ (Transformation|GetWorldLocation _mesh) (Math|Vector|MakeVector (Math|Conversions|ToFloat(Integer) _returnvalue) (Math|Conversions|ToFloat(Integer) _returnvalue) (Math|Conversions|ToFloat(Integer) _returnvalue))) (Transformation|GetWorldRotation _mesh))))
  (CallFunction|DumbPlayerFollow))

(event Custom|predie
  ;[0.15 0.15 0.15 0.5] Health and damage
  (CallFunction|Die))

(event Custom|Attack
  (bind _staticmesh (Variables|Default|GetStaticMesh))
  (Variables|Default|Setcurrent%20scale (Variables|/Script/Engine.SceneComponent|GetRelativeScale3D _staticmesh))
  (Audio|PlaySoundatLocation "/Game/Imported/Audio/FX/Actions/Swoosh.Swoosh" (Transformation|GetWorldLocation _staticmesh) "0, 0, 0" 3.0 1.1 0.0 0 0 0 0)
  (bind (_direction _newtrack_0 _newtrack_1) (Timeline|Timeline PlayFromStart)
    (:Update
      (Transformation|AddLocalOffset (Variables|Collision|GetCapsuleComponent) (Math|Vector|MakeVector 0.0 0.0 (* _newtrack_1 3e+01)) false false)
      (Transformation|SetRelativeScale3D (Variables|Default|GetStaticMesh) (Math|Vector|Lerp(Vector) (Variables|Default|Getcurrent%20scale) (* (Variables|Default|Getcurrent%20scale) "0.250000,0.250000,1.750000") _newtrack_0)))
    (:Finished
      (if (< (Math|Vector|Distance(Vector) (Transformation|GetWorldLocation (Variables|Collision|GetCapsuleComponent)) (Class|CharacterMovementComponent|GetLastUpdateLocation (Variables|/Script/Engine.Character|GetCharacterMovement (Game|GetPlayerCharacter 0)))) (Variables|Default|GetMeleRange))
        ;[0.15 0.15 0.15 0.5] Multiplayer is non existant
        (bind _outactors (Actor|GetAllActorsOfClass "/Game/FirstPerson/Blueprints/BP_FirstPersonCharacter.BP_FirstPersonCharacter_C"))
        (Default|TakeDamage _outactors 1)
        (bind _newtrack_0_2 (Timeline|Timeline_0 PlayFromStart)
          (:Update
            (Transformation|SetRelativeScale3D (Variables|Default|GetStaticMesh) (Math|Vector|Lerp(Vector) (Variables|Default|Getcurrent%20scale) (* (Variables|Default|Getcurrent%20scale) "0.250000,0.250000,1.750000") _newtrack_0_2))))
        (else
          (Timeline|Timeline_0 PlayFromStart))))))

(event Custom|HighJump
  (bind _current_scale (Variables|Default|Getcurrent%20scale))
  (bind _current_scale_2 (Variables|Default|Getcurrent%20scale))
  (Utilities|FlowControl|DoOnce false :!label _label
    (:Completed
      (bind (_direction _newtrack_0 _newtrack_1) (Timeline|Timeline_1 Play)
        (:Update
          (Transformation|AddLocalOffset (Variables|Collision|GetCapsuleComponent) (Math|Vector|MakeVector 0.0 0.0 (* _newtrack_1 1e+02)) false false)
          (Transformation|SetRelativeScale3D (Variables|Default|GetStaticMesh) (Math|Vector|Lerp(Vector) _current_scale_2 (* _current_scale_2 "0.250000,0.250000,1.750000") _newtrack_0))
          (bind _newtrack_0_2 (Timeline|Timeline_2 PlayFromStart)
            (:Update
              (Transformation|SetRelativeScale3D (Variables|Default|GetStaticMesh) (Math|Vector|Lerp(Vector) _current_scale (* _current_scale "0.250000,0.250000,1.750000") _newtrack_0_2))
              (Utilities|FlowControl|Delay 0.2)
              (goto _label Reset))))))))

(event EventBeginPlay
  (Utilities|FlowControl|Delay 0.2)
  (Variables|/Script/Engine.CharacterMovementComponent|SetMaxWalkSpeed (Variables|Character|GetCharacterMovement) 2e+02)
  (Variables|Default|SetLocalhealth (Variables|Default|GetHealth))
  (CallFunction|DumbPlayerFollow))

(event Collision|EventActorBeginOverlap
  (params (OtherActor :type Actor%20Object%20Reference)))

(event EventTick
  (params (DeltaSeconds :type Float%20%28single-precision%29)))

(event EventGetManager
  (params (Manager :type BP%20Enemy%20Spawn%20Manager%20Object%20Reference))
  (Variables|Default|SetManager Manager))

(fn ConstructionScript)